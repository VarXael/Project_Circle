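; Enemy for the RhythmBeater showcase that fires a single projectile at the boxing player character.
; On BeginPlay it finds the player, turns to face their first-person camera and calls ShootGun.
; ShootGun spawns a BP_EnemyRhythm_Projectile at ProjectileStartPos, passing itself and the player reference, and stores the result.
; The ReturnedToTheSender event destroys the enemy.
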(event `self.ReceiveBeginPlay`
  (bind _returnvalue (`GameplayStatics.GetActorOfClass` "/Game/TechShowcase/RhythmBeater/Blueprints/BP_BoxingPlayerCharacter.BP_BoxingPlayerCharacter_C"))
  (`KismetSystemLibrary.PrintString` (`KismetSystemLibrary.GetDisplayName` _returnvalue))
  (set `self.PlayerRef` _returnvalue)
  (`self.K2_SetActorRotation` (`KismetMathLibrary.FindLookAtRotation` (`SceneComponent.K2_GetComponentLocation` (`self.CapsuleComponent`)) (`SceneComponent.K2_GetComponentLocation` (`/Game/TechShowcase/RhythmBeater/Blueprints/BP_BoxingPlayerCharacter.FirstPersonCamera` _returnvalue))))
  (`self.ShootGun`))

(event `ShootGun`
  (bind _returnvalue (`|SpawnActorFromClass` "/Game/TechShowcase/RhythmBeater/Blueprints/BP_EnemyRhythm_Projectile.BP_EnemyRhythm_Projectile_C" (`SceneComponent.K2_GetComponentToWorld` (`self.ProjectileStartPos`)) "AlwaysSpawn" "MultiplyWithRoot" self self (`self.PlayerRef`) self))
  (set `self.ProjectileShot` _returnvalue))

(event `ReturnedToTheSender`
  (`self.K2_DestroyActor`))

(fn `UserConstructionScript`)