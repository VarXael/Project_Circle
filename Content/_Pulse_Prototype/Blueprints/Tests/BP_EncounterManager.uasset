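; Test encounter manager that drives enemy dummies from music note hits.
; On BeginPlay it caches every BP_Enemy_Test and binds to the music analysis subsystem's note-hit and song-progress events.
; Each note hit forwards OnNoteHit to one random cached enemy; the RandomInteger(Length - 1) index never selects the last one.
; The song-progress handler is empty, and the pattern turret beat-shot call is disconnected.
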(event `self.ReceiveBeginPlay`
  (bind _returnvalue (subsystem `PcMusicAnalysisSubsystem`))
  (bind _outactors (`GameplayStatics.GetAllActorsOfClass` "/Game/Slide_Prototype/Core/Enemies/EnemyTypes/BP_Enemy_Test.BP_Enemy_Test_C"))
  (set `self.EnemyDummies` _outactors)
  (add `PcMusicAnalysisSubsystem.OnNoteHit` _returnvalue (delegate `OnNoteHit`))
  (add `PcMusicAnalysisSubsystem.OnSongProgress` _returnvalue (delegate `OnSongProgress_Event`)))

(event `OnSongProgress_Event`
  (params (CurrentSongProgress :type "Float (single-precision)")))

(event `OnNoteHit`
  (params (TimestampMS :type Integer) (NoteType :type Integer) (HitSound :type Integer))
  (`|ExecutionSequence`
    (:`then_0`
      (if (`KismetArrayLibrary.Array_IsValidIndex` (`self.EnemyDummies`))
        (`/Game/Slide_Prototype/Core/Enemies/EnemyTypes/BP_Enemy_Test.OnNoteHit` (`|GetArrayItem` (`self.EnemyDummies`) (`KismetMathLibrary.RandomInteger` (- (`KismetArrayLibrary.Array_Length` (`self.EnemyDummies`)) 1))))))))

(fn `UserConstructionScript`)