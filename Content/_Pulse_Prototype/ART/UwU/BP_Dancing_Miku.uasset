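; BP_Dancing_Miku is a prototype dancer Blueprint that reacts to note hits from the music analysis subsystem.
; On BeginPlay it binds to the subsystem's OnNoteHit event.
; Each hit advances PoseIndex by a random one or two steps modulo three, so it never repeats, and prints the result.
; The graph does not apply the index to the skeletal mesh, and its leader-pose call is unconnected.
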(event `self.ReceiveBeginPlay`
  (add `PcMusicAnalysisSubsystem.OnNoteHit` (subsystem `PcMusicAnalysisSubsystem`) (delegate `OnNoteHit_Event`)))

(event `OnNoteHit_Event`
  (params (TimestampMS :type Integer) (NoteType :type Integer) (HitSound :type Integer))
  (bind _output_get (set `self.PoseIndex` (mod (+ (`self.PoseIndex`) (`KismetMathLibrary.RandomIntegerInRange` 1 2)) 3)))
  (`KismetSystemLibrary.PrintString` (`KismetStringLibrary.Conv_IntToString` _output_get)))

(fn `UserConstructionScript`)