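; BP_PlayerCharacter is the player character for the Slide_Prototype game, serving as the binding layer for player input.
; Enhanced Input actions for look, move, jump, primary fire, laser secondary fire and drift each forward to an Input function not defined here.
; Primary fire and drift use Started and Completed to begin and end their actions.
; BeginPlay and the construction script are empty, and experimental HUD and skate widget creation is left disconnected.
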(event `self.ReceiveBeginPlay`)

(event `EnhancedInput|/Game/Slide_Prototype/Core/Player/Input/Actions/IA_Look`
  (params (ActionValue :type "Vector2D Structure") (ElapsedSeconds :type "Float (double-precision)") (TriggeredSeconds :type "Float (double-precision)") (InputAction :type "InputAction Object Reference" :default "/Game/Slide_Prototype/Core/Player/Input/Actions/IA_Look.IA_Look"))
  (:`Triggered`
    (`self.Input_Look` ActionValue)))

(event `EnhancedInput|/Game/Slide_Prototype/Core/Player/Input/Actions/IA_Move`
  (params (ActionValue :type "Vector2D Structure") (ElapsedSeconds :type "Float (double-precision)") (TriggeredSeconds :type "Float (double-precision)") (InputAction :type "InputAction Object Reference" :default "/Game/Slide_Prototype/Core/Player/Input/Actions/IA_Move.IA_Move"))
  (:`Triggered`
    (`self.Input_Move` ActionValue)))

(event `EnhancedInput|/Game/Slide_Prototype/Core/Player/Input/Actions/IA_Jump`
  (params (ActionValue :type Boolean) (ElapsedSeconds :type "Float (double-precision)") (TriggeredSeconds :type "Float (double-precision)") (InputAction :type "InputAction Object Reference" :default "/Game/Slide_Prototype/Core/Player/Input/Actions/IA_Jump.IA_Jump"))
  (:`Triggered`
    (`self.Input_JumpTrigger`)))

(event `EnhancedInput|/Game/Slide_Prototype/Core/Player/Input/Actions/IA_PrimaryFire`
  (params (ActionValue :type Boolean) (ElapsedSeconds :type "Float (double-precision)") (TriggeredSeconds :type "Float (double-precision)") (InputAction :type "InputAction Object Reference" :default "/Game/Slide_Prototype/Core/Player/Input/Actions/IA_PrimaryFire.IA_PrimaryFire"))
  (:`Started`
    (`self.Input_StartAttack`))
  (:`Completed`
    (`self.Input_StopAttack`)))

(event `EnhancedInput|/Game/Slide_Prototype/Core/Player/Input/Actions/IA_SecondaryFire`
  (params (ActionValue :type Boolean) (ElapsedSeconds :type "Float (double-precision)") (TriggeredSeconds :type "Float (double-precision)") (InputAction :type "InputAction Object Reference" :default "/Game/Slide_Prototype/Core/Player/Input/Actions/IA_SecondaryFire.IA_SecondaryFire"))
  (:`Triggered`
    (`self.Input_FireLaser`)))

(event `EnhancedInput|/Game/Slide_Prototype/Core/Player/Input/Actions/IA_Drift`
  (params (ActionValue :type Boolean) (ElapsedSeconds :type "Float (double-precision)") (TriggeredSeconds :type "Float (double-precision)") (InputAction :type "InputAction Object Reference" :default "/Game/Slide_Prototype/Core/Player/Input/Actions/IA_Drift.IA_Drift"))
  (:`Started`
    (`self.Input_StartDrift`))
  (:`Completed`
    (`self.Input_StopDrift`)))

(fn `UserConstructionScript`)