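; Base enemy Blueprint that reacts to note hits with a visual pulse, a sound and a shot.
; OnNoteHit enlarges the cube, tints its dynamic material red, plays a clap sound and calls Shoot, whose logic is not in this graph.
; Tick constantly interpolates scale and color back to normal size and white, so each hit reads as a brief flash.
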(event `self.ReceiveTick`
  (params (DeltaSeconds :type "Float (single-precision)"))
  (bind _cube (`self.Cube`))
  (`SceneComponent.SetRelativeScale3D` _cube (`KismetMathLibrary.VInterpTo_Constant` (`SceneComponent.K2_GetComponentScale` _cube) (1.0 1.0 1.0) DeltaSeconds 3.0))
  (bind _returnvalue (`MaterialInstanceDynamic.K2_GetVectorParameterValue` (`self.BodyDynamicMaterial`) "Color"))
  (bind (_r _g _b) (`KismetMathLibrary.BreakColor` _returnvalue))
  (bind (_returnvalue_x _returnvalue_y _returnvalue_z) (`KismetMathLibrary.BreakVector` (`KismetMathLibrary.VInterpTo_Constant` (`KismetMathLibrary.MakeVector` _r _g _b) (1.0 1.0 1.0) (`GameplayStatics.GetWorldDeltaSeconds`) 3.0)))
  (`MaterialInstanceDynamic.SetVectorParameterValue` (`self.BodyDynamicMaterial`) "Color" (`KismetMathLibrary.MakeColor` _returnvalue_x _returnvalue_y _returnvalue_z)))

(event `self.ReceiveBeginPlay`
  (bind _cube (`self.Cube`))
  (bind _returnvalue (`PrimitiveComponent.CreateDynamicMaterialInstance` _cube 0 (`PrimitiveComponent.GetMaterial` _cube 0) "None"))
  (set `self.BodyDynamicMaterial` _returnvalue))

(event `OnNoteHit`
  (`SceneComponent.SetRelativeScale3D` (`self.Cube`) (1.5 1.5 1.5))
  (`GameplayStatics.PlaySound2D` "/Game/soft-hitclap.soft-hitclap" 0.5 1.0 0.0 null null)
  (`MaterialInstanceDynamic.SetVectorParameterValue` (`self.BodyDynamicMaterial`) "Color" (struct :`R` 1.0 :`A` 1.0))
  (`self.Shoot`))

(fn `UserConstructionScript`)