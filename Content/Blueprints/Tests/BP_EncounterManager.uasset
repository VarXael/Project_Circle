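; BP_EncounterManager is a test manager that makes enemies react to musical notes.
; On BeginPlay it caches all BP_Enemy_Base actors and binds to the PcMusicAnalysisSubsystem's note-hit and song-progress events.
; Each note hit calls OnNoteHit on a random cached enemy, though the Length-1 random bound excludes the last one when several exist.
; The song-progress handler is an empty stub.
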(event `self.ReceiveBeginPlay`
  (bind _returnvalue (subsystem `PcMusicAnalysisSubsystem`))
  (bind _outactors (`GameplayStatics.GetAllActorsOfClass` "/Game/_Prototype/Core/Enemies/EnemyTypes/BP_Enemy_Base.BP_Enemy_Base_C"))
  (set `self.EnemyDummies` _outactors)
  (add `PcMusicAnalysisSubsystem.OnNoteHit` _returnvalue (delegate `OnNoteHit`))
  (add `PcMusicAnalysisSubsystem.OnSongProgress` _returnvalue (delegate `OnSongProgress_Event`)))

(event `OnSongProgress_Event`
  (params (CurrentSongProgress :type "Float (single-precision)")))

(event `OnNoteHit`
  (params (TimestampMS :type Integer) (NoteType :type Integer) (HitSound :type Integer))
  (if (`KismetArrayLibrary.Array_IsValidIndex` (`self.EnemyDummies`))
    (`/Game/_Prototype/Core/Enemies/EnemyTypes/BP_Enemy_Base.OnNoteHit` (`|GetArrayItem` (`self.EnemyDummies`) (`KismetMathLibrary.RandomInteger` (- (`KismetArrayLibrary.Array_Length` (`self.EnemyDummies`)) 1))))))

(fn `UserConstructionScript`)