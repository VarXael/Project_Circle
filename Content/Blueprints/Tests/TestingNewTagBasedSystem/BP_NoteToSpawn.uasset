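; BP_NoteToSpawn is a short-lived note actor that shows an approaching-circle effect through its WBP_Note widget.
; On BeginPlay it applies a dynamic M_ApproachingCircle material to the widget's image, then destroys itself after a brief delay.
; Tick drives the material's ApproachingTime parameter toward one at constant speed.
; An unconnected render-visibility debug print remains in the graph.
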(event `self.ReceiveBeginPlay`
  (bind _aswbp_note (cast `/Game/Blueprints/Tests/WBP_Note` (`WidgetComponent.GetUserWidgetObject` (`self.Widget`))))
  (bind _returnvalue (`KismetMaterialLibrary.CreateDynamicMaterialInstance` "/Game/Blueprints/Tests/M_ApproachingCircle.M_ApproachingCircle"))
  (bind _output_get (set `self.NoteMaterialInst` _returnvalue))
  (`Image.SetBrushFromMaterial` (`/Game/Blueprints/Tests/WBP_Note.Image_56` _aswbp_note) _output_get)
  (`KismetSystemLibrary.Delay` 0.6)
  (`self.K2_DestroyActor`))

(event `self.ReceiveTick`
  (params (DeltaSeconds :type "Float (single-precision)"))
  (bind _notematerialinst (`self.NoteMaterialInst`))
  (bind _returnvalue (`MaterialInstanceDynamic.K2_GetScalarParameterValue` _notematerialinst "ApproachingTime"))
  (`MaterialInstanceDynamic.SetScalarParameterValue` _notematerialinst "ApproachingTime" (`KismetMathLibrary.FInterpTo_Constant` _returnvalue 1.0 DeltaSeconds 1.5)))

(event `self.ReceiveActorBeginOverlap`
  (params (OtherActor :type "Actor Object Reference")))

(fn `UserConstructionScript`)