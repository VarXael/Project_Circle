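; BP_MusicSphere is a test actor that visualizes music events with two components, Green and Red, plus sound cues.
; Beat hits play a drum sound and snap Green to an offset from its start; Tick eases only Z back, leaving X/Y displaced.
; Note hits play a clap and enlarge Red, which Tick shrinks to unit scale at constant speed.
; Beat drops swap Green's material according to the music section type.
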(event `OnHitBeat`
  (`GameplayStatics.PlaySound2D` "/Game/drum-hitnormal.drum-hitnormal" 1.0 1.0 0.0 null null)
  (`SceneComponent.K2_SetWorldLocation` (`self.Green`) (+ (`self.StartObjectPos`) (-50.0 -50.0 -50.0)) false true))

(event `self.ReceiveBeginPlay`
  (set `self.StartObjectPos` (`SceneComponent.K2_GetComponentLocation` (`self.Green`))))

(event `OnNoteHit`
  (`SceneComponent.SetRelativeScale3D` (`self.Red`) (2.0 2.0 2.0))
  (`GameplayStatics.PlaySound2D` "/Game/soft-hitclap.soft-hitclap" 1.0 1.0 0.0 null null))

(event `self.ReceiveTick`
  (params (DeltaSeconds :type "Float (single-precision)"))
  (bind _green (`self.Green`))
  (bind (_returnvalue_x _returnvalue_y) (`KismetMathLibrary.BreakVector` (`SceneComponent.K2_GetComponentLocation` _green)))
  (bind (_returnvalue_x_2 _returnvalue_y_2 _returnvalue_z) (`KismetMathLibrary.BreakVector` (`KismetMathLibrary.VInterpTo` (`SceneComponent.K2_GetComponentLocation` (`self.Green`)) (`self.StartObjectPos`) DeltaSeconds 10.0)))
  (`SceneComponent.SetRelativeScale3D` (`self.Red`) (`KismetMathLibrary.VInterpTo_Constant` (`SceneComponent.K2_GetComponentScale` (`self.Red`)) (1.0 1.0 1.0) DeltaSeconds 3.0))
  (`SceneComponent.K2_SetWorldLocation` _green (`KismetMathLibrary.MakeVector` _returnvalue_x _returnvalue_y _returnvalue_z) false true))

(event `OnBeatDrop`
  (params (NewParam :type "EPcGameplaySectionType Enum" :default "Normal"))
  (switch `EPcGameplaySectionType` NewParam
    (:`Normal`
      (`PrimitiveComponent.SetMaterial` (`self.Green`) 0 "/Game/Blueprints/Tests/M_MaterialColor_0.M_MaterialColor_0"))
    (:`HighEnergy`
      (`PrimitiveComponent.SetMaterial` (`self.Green`) 0 "/Game/Blueprints/Tests/M_MaterialColor_1.M_MaterialColor_1"))
    (:`Buildup`
      (`PrimitiveComponent.SetMaterial` (`self.Green`) 0 "/Game/Default_FirstPersonContent/FPWeapon/Materials/M_FPGun.M_FPGun"))
    (:`Cooldown`
      (`PrimitiveComponent.SetMaterial` (`self.Green`) 0 "/Game/Default_FirstPersonContent/FPWeapon/Materials/FirstPersonProjectileMaterial.FirstPersonProjectileMaterial"))
    (:`Break`
      (`PrimitiveComponent.SetMaterial` (`self.Green`) 0 "/Game/Default_FirstPersonContent/LevelPrototyping/Materials/MI_PrototypeGrid_TopDark.MI_PrototypeGrid_TopDark"))))

(fn `UserConstructionScript`)