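; BP_MusicSphere is a music-reactive sphere that bobs, pulses and changes material with the current song.
; Tick moves it vertically around its BeginPlay height using a cosine of song BPM and progress, so the bob follows the tempo.
; OnHitBeat snaps the actor to double scale, and Tick interpolates it back to normal.
; OnBeatDrop swaps between two materials depending on whether the section is Kiai.
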(event `self.ReceiveTick`
  (params (DeltaSeconds :type "Float (single-precision)"))
  (bind (_startobjectpos_x _startobjectpos_y _startobjectpos_z) (`KismetMathLibrary.BreakVector` (`self.StartObjectPos`)))
  (bind (_returnvalue_x _returnvalue_y) (`KismetMathLibrary.BreakVector` (`SceneComponent.K2_GetComponentLocation` (`self.Sphere`))))
  (`|ExecutionSequence`
    (:`then_0`
      (`self.SetActorScale3D` (`KismetMathLibrary.VInterpTo` (`SceneComponent.K2_GetComponentScale` (`self.Sphere`)) (1.0 1.0 1.0) DeltaSeconds 1.0))
      (`self.K2_SetActorLocation` (`KismetMathLibrary.MakeVector` _returnvalue_x _returnvalue_y (+ _startobjectpos_z (* (`KismetMathLibrary.Cos` (* (* (/ (`KismetMathLibrary.MultiplyByPi` 1.0) 30.0) (`self.CurrentSongBPM`)) (`self.CurrentSongProgress`))) 20.0))) false true))))

(event `OnBeatDrop`
  (params (bIsKiai :type Boolean))
  (`PrimitiveComponent.SetMaterial` (`self.Sphere`) 0 (select `bool` bIsKiai :`false` "/Game/Blueprints/M_MaterialColor_0.M_MaterialColor_0" :`true` "/Game/Blueprints/M_MaterialColor_1.M_MaterialColor_1" :!type "MaterialInterface Object Reference")))

(event `OnHitBeat`
  (`self.SetActorScale3D` (2.0 2.0 2.0)))

(event `self.ReceiveBeginPlay`
  (set `self.StartObjectPos` (`SceneComponent.K2_GetComponentLocation` (`self.Sphere`))))

(fn `UserConstructionScript`)