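; BP_SpawnProxy is a gameplay ability that spawns a BP_MusicProxy actor in front of the player's camera.
; On activation it places the proxy a short fixed distance along the camera manager's forward vector, with zero rotation and unit scale.
; A validity check prints a debug string for success or failure.
; The graph never calls EndAbility, and the end event is an unused stub.
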(event `self.K2_ActivateAbility`
  (bind _returnvalue (`GameplayStatics.GetPlayerCameraManager` 0))
  (bind _returnvalue_2 (`|SpawnActorFromClass` "/Game/Blueprints/Tests/BP_MusicProxy.BP_MusicProxy_C" (`KismetMathLibrary.MakeTransform` (+ (`PlayerCameraManager.GetCameraLocation` _returnvalue) (* (`Actor.GetActorForwardVector` _returnvalue) 100.0))) "Undefined" "MultiplyWithRoot" null null))
  (if (`KismetSystemLibrary.IsValid` _returnvalue_2)
    (`KismetSystemLibrary.PrintString` "Spawned")
    (else
      (`KismetSystemLibrary.PrintString` "NOTTTTTTTTT"))))